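; Game Instance that handles the PlayFab backend for Battle Drones: accounts, inventory, matchmaking and currency rewards.
; Clients initialize the SDK, log in by email with username fallback, then show the lobby and load currency and owned characters.
; Matchmaking creates a ticket, polls it by looping timer, then opens the allocated server's IP and port, passing name and team as URL options.
; Dedicated servers skip PlayFab setup and quit after twenty minutes.
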(event `self.ReceiveInit`
  (bind _playfabsetting_gametitleid (break `/Game/BattleDronesMultiplayer/Blueprints/GameSettings/Utilities/S_PlayfabSetting` (`self.PlayfabSetting`)))
  ;[1 1 1] Get Playfab server from ID
  (if (`KismetSystemLibrary.IsDedicatedServer`)
    (`parent.ReceiveInit`)
    (`KismetSystemLibrary.Delay` 1200.0)
    (`KismetSystemLibrary.QuitGame` null "Quit")
    (else
      (`PlayFabUtilities.setPlayFabSettings` _playfabsetting_gametitleid))))

(event `RegisterUser`
  (params (Email :type String) (Username :type String) (Password :type String))
  (`KismetSystemLibrary.PrintString` "Please wait..." true true (struct :`G` 1.0 :`A` 1.0))
  (`PlayFabClientAPI.RegisterPlayFabUser` (make `ClientRegisterPlayFabUserRequest` null Username Email "" null Password "" false Username) (`|CreateDelegate` :!event `OnRegisterSuccess`) (`|CreateDelegate` :!event `OnFailure`)))

(event `LoginUser`
  (params (Email :type String) (Password :type String))
  (bind (_useraccount_email _useraccount_username _useraccount_password) (break `/Game/BattleDronesMultiplayer/Blueprints/GameSettings/Utilities/S_UserAccount` (`self.UserAccount`)))
  (`KismetSystemLibrary.PrintString` "Please wait..." true true (struct :`G` 1.0 :`A` 1.0))
  (bind (_response _customdata _successful) (`PlayFabClientAPI.LoginWithEmailAddress` (make `ClientLoginWithEmailAddressRequest` null Email null Password) (`|CreateDelegate` :!event `OnLoginSuccess`) (delegate `Info - TryWithUsername`))
    (:`OnPlayFabResponse`
      (if (not _successful)
        (`PlayFabClientAPI.LoginWithPlayFab` (make `ClientLoginWithPlayFabRequest` null null _useraccount_password _useraccount_username) (`|CreateDelegate` :!event `OnLoginSuccess`) (`|CreateDelegate` :!event `OnFailure`))))))

(event `RecoverAccount`
  (params (Email :type String))
  (`PlayFabClientAPI.SendAccountRecoveryEmail` (make `ClientSendAccountRecoveryEmailRequest` null Email) (`|CreateDelegate` :!event `OnAccountRecovery`) (`|CreateDelegate` :!event `OnFailure`)))

(event `OnFailure`
  (params (error :type "PlayFabError Structure") (customData :type "Object Object Reference"))
  (`KismetSystemLibrary.PrintString` (`KismetStringLibrary.Concat_StrStr` error_ErrorName " | " error_ErrorDetails)))

(event `OnRegisterSuccess`
  (params (result :type "ClientRegisterPlayFabUserResult Structure") (customData :type "Object Object Reference"))
  (setmembers `/Game/BattleDronesMultiplayer/Blueprints/GameSettings/Utilities/S_UserAccount` :`StructRef` (`self.UserAccount`) :`PlayfabId` (`.PlayFabId` (break `ClientRegisterPlayFabUserResult` result)))
  (`KismetSystemLibrary.PrintString` "Registered Successfully." true true (struct :`R` 1.0 :`G` 1.0 :`B` 0.5 :`A` 1.0))
  (if (`Widget.IsInViewport` (`self.AuthPage_Ref`)) :!label _label
    (`Widget.RemoveFromParent` (`self.AuthPage_Ref`))
    (`self.ShowLobbyPage`)))

(event `OnLoginSuccess`
  (params (result :type "ClientLoginResult Structure") (customData :type "Object Object Reference"))
  (setmembers `/Game/BattleDronesMultiplayer/Blueprints/GameSettings/Utilities/S_UserAccount` :`StructRef` (`self.UserAccount`) :`PlayfabId` (`.PlayFabId` (break `ClientLoginResult` result)))
  (`KismetSystemLibrary.PrintString` "Login Successfully." true true (struct :`R` 1.0 :`G` 1.0 :`B` 0.5 :`A` 1.0))
  (goto _label))

(event `OnAccountRecovery`
  (params (result :type "ClientSendAccountRecoveryEmailResult Structure") (customData :type "Object Object Reference"))
  (`KismetSystemLibrary.PrintString` "Account recovery sent"))

(event `Info - TryWithUsername`
  (params (error :type "PlayFabError Structure") (customData :type "Object Object Reference"))
  (`KismetSystemLibrary.PrintString` "Email not found. Trying with Username."))

(event `SavePlayerInfo`
  (params (Email :type String) (Username :type String) (Password :type String))
  (setmembers `/Game/BattleDronesMultiplayer/Blueprints/GameSettings/Utilities/S_UserAccount` :`StructRef` (`self.UserAccount`) :`Email` Email :`Username` Username :`Password` Password))

(event `ShowAuthPage`
  (`self.AuthPage_Ref`
    (:`then`
      _)
    (:`else`
      (bind _returnvalue (`|CreateWidget` "/Game/BattleDronesMultiplayer/Blueprints/UI/Login/W_LoginInterface.W_LoginInterface_C"))
      (set `self.AuthPage_Ref` _returnvalue)))
  (`UserWidget.AddToViewport` (`self.AuthPage_Ref`) 0))

(event `ShowLobbyPage`
  (`self.LobbyPage_Ref`
    (:`then`
      _)
    (:`else`
      (bind _returnvalue (`|CreateWidget` "/Game/BattleDronesMultiplayer/Blueprints/UI/W_Lobby.W_Lobby_C"))
      (set `self.LobbyPage_Ref` _returnvalue)))
  (`UserWidget.AddToViewport` (`self.LobbyPage_Ref`) 0)
  (`self.GetInventory`))

(event `ShowInventoryPage`
  (`self.InventoryPage_Ref`
    (:`then`
      _)
    (:`else`
      (bind _returnvalue (`|CreateWidget` "/Game/BattleDronesMultiplayer/Blueprints/UI/W_Inventory.W_Inventory_C"))
      (set `self.InventoryPage_Ref` _returnvalue)))
  (`UserWidget.AddToViewport` (`self.InventoryPage_Ref`) 0))

(event `GetInventory`
  (`PlayFabClientAPI.GetUserInventory` (make `ClientGetUserInventoryRequest` null) (delegate `GetUserInventoryOnSuccessForCurrency`) (`|CreateDelegate` :!event `OnFailure`)))

(event `GetUserInventoryOnSuccessForCurrency`
  (params (result :type "ClientGetUserInventoryResult Structure") (customData :type "Object Object Reference"))
  (bind (_playfabsetting_gametitleid _playfabsetting_secretapikey _playfabsetting_currencyname) (break `/Game/BattleDronesMultiplayer/Blueprints/GameSettings/Utilities/S_PlayfabSetting` (`self.PlayfabSetting`)))
  (`|ExecutionSequence`
    (:`then_0`
      (setmembers `/Game/BattleDronesMultiplayer/Blueprints/GameSettings/Utilities/S_UserAccount` :`StructRef` (`self.UserAccount`) :`Currency` (`KismetMathLibrary.FTrunc` (`PlayFabJsonObject.GetNumberField` result_VirtualCurrency _playfabsetting_currencyname))))
    (:`then_1`
      (for _array_element result_Inventory
        (switch `string` (`PlayFabJsonObject.GetStringField` _array_element "ItemId")
          (:`Character1`
            (`KismetArrayLibrary.Array_Set` (`self.Characters`) 0 true))
          (:`Character2`
            (`KismetArrayLibrary.Array_Set` (`self.Characters`) 1 true))
          (:`Character3`
            (`KismetArrayLibrary.Array_Set` (`self.Characters`) 2 true))
          (:`Character4`
            (`KismetArrayLibrary.Array_Set` (`self.Characters`) 3 true))
          (:`Character5`
            (`KismetArrayLibrary.Array_Set` (`self.Characters`) 4 true)))))))

(event `GetAccountInfo`
  (`PlayFabClientAPI.GetAccountInfo` (make `ClientGetAccountInfoRequest` :`PlayFabId` (`.PlayfabId_12_9E46C7BD4FE41D8F52D596B86600F81F` (break `/Game/BattleDronesMultiplayer/Blueprints/GameSettings/Utilities/S_UserAccount` (`self.UserAccount`)))) (delegate `GetAccountInfoOnSuccess`) (`|CreateDelegate` :!event `OnFailure`)))

(event `GetAccountInfoOnSuccess`
  (params (result :type "ClientGetAccountInfoResult Structure") (customData :type "Object Object Reference"))
  (`|ExecutionSequence`
    (:`then_0`
      (setmembers `/Game/BattleDronesMultiplayer/Blueprints/GameSettings/Utilities/S_UserAccount` :`StructRef` (`self.UserAccount`) :`TitlePlayerAccountId` (`PlayFabJsonObject.GetStringField` (`PlayFabJsonObject.GetObjectField` (`PlayFabJsonObject.GetObjectField` (`.AccountInfo` (break `ClientGetAccountInfoResult` result)) "TitleInfo") "TitlePlayerAccount") "Id")))
    (:`then_1`
      (`self.BeforeCreateMatchmakingTicket`))))

(event `BeforeCreateMatchmakingTicket`
  (bind _returnvalue (`PlayFabJsonObject.ConstructJsonObject`))
  (bind _latencynortheurope (`self.LatencyNorthEurope`))
  (bind _latencyeastus (`self.LatencyEastUs`))
  (bind _entitykeysettings (`self.EntityKeySettings`))
  (`|ExecutionSequence`
    (:`then_0`
      (`KismetSystemLibrary.PrintString` "Ready to create matchmaking ticket" true true (struct :`R` 0.5 :`G` 1.0 :`B` 0.5 :`A` 1.0))
      (`DestroySessionCallbackProxy.DestroySession` (`GameplayStatics.GetPlayerController` 0)
        (:`then`
          (set `self.CreatorSettings` (`PlayFabJsonObject.ConstructJsonObject`))
          (set `self.EntityKeySettings` (`PlayFabJsonObject.ConstructJsonObject`))
          (set `self.AttributesSetting` (`PlayFabJsonObject.ConstructJsonObject`))
          (set `self.LatencyEastUs` _returnvalue)
          (set `self.LatencyNorthEurope` _returnvalue)
          (set `self.Latencies` (`PlayFabJsonObject.ConstructJsonObject`)))))
    (:`then_1`
      (`PlayFabJsonObject.SetStringField` _entitykeysettings "Id" (`.TitlePlayerAccountId_15_8D16608C408A11DCCB376A8CD5D80432` (break `/Game/BattleDronesMultiplayer/Blueprints/GameSettings/Utilities/S_UserAccount` (`self.UserAccount`))))
      (`PlayFabJsonObject.SetStringField` _entitykeysettings "Type" "title_player_account")
      (`PlayFabJsonObject.SetStringField` _entitykeysettings "TypeString" "title_player_account")
      (`PlayFabJsonObject.SetObjectField` (`self.CreatorSettings`) "Entity" (`self.EntityKeySettings`))
      (`PlayFabJsonObject.SetStringField` _latencyeastus "region" "EastUs")
      (`PlayFabJsonObject.SetStringField` _latencyeastus "latency" "150")
      (`PlayFabJsonObject.SetStringField` _latencynortheurope "region" "WestUs")
      (`PlayFabJsonObject.SetStringField` _latencynortheurope "latency" "100")
      (`PlayFabJsonObject.SetArrayField` (`self.Latencies`) "latencies" (`|MakeArray` (`PlayFabJsonValue.ConstructJsonValueObject` (`self.LatencyEastUs`)) (`PlayFabJsonValue.ConstructJsonValueObject` (`self.LatencyNorthEurope`))))
      (`PlayFabJsonObject.SetObjectField` (`self.AttributesSetting`) "DataObject" (`self.Latencies`))
      (`PlayFabJsonObject.SetObjectField` (`self.CreatorSettings`) "Attributes" (`self.AttributesSetting`)))
    (:`then_2`
      (`PlayFabMultiplayerAPI.CancelAllMatchmakingTicketsForPlayer` (make `MultiplayerCancelAllMatchmakingTicketsForPlayerRequest` :`Entity` (`self.EntityKeySettings`) :`QueueName` (`self.QueueName`)) (delegate `SuccessCancelAllMatchmakingTicketsForPlayer`) (`|CreateDelegate` :!event `OnFailure`)))))

(event `SuccessCreateMatchmakingTicket`
  (params (result :type "MultiplayerCreateMatchmakingTicketResult Structure") (customData :type "Object Object Reference"))
  (set `self.TicketId` (`.TicketId` (break `MultiplayerCreateMatchmakingTicketResult` result)))
  (bind _returnvalue (`KismetSystemLibrary.K2_SetTimer` null "CheckIfMatchFound" 5.0 true))
  (set `self.SearchingTimerHandler` _returnvalue)
  (`KismetSystemLibrary.PrintString` "Matchmaking ticket created!" true true (struct :`R` 1.0 :`B` 0.5 :`A` 1.0))
  (`KismetSystemLibrary.PrintString` "Searching..." true true (struct :`G` 1.0 :`B` 0.5 :`A` 1.0) 4.5))

(event `GetMatchmakingTicket`
  (`PlayFabMultiplayerAPI.GetMatchmakingTicket` (make `MultiplayerGetMatchmakingTicketRequest` :`QueueName` (`self.QueueName`) :`TicketId` (`self.TicketId`)) (delegate `SuccessGetMatchmakingTicket`) (`|CreateDelegate` :!event `OnFailure`)))

(event `SuccessGetMatchmakingTicket`
  (params (result :type "MultiplayerGetMatchmakingTicketResult Structure") (customData :type "Object Object Reference"))
  (bind (_cancellationreasonstring _created _creator _giveupafterseconds _matchid _members _memberstomatchwith _queuename _status) (break `MultiplayerGetMatchmakingTicketResult` result))
  (if (== _status "Matched")
    (`KismetSystemLibrary.K2_ClearAndInvalidateTimerHandle` (`self.SearchingTimerHandler`))
    (set `self.MatchId` _matchid)
    (`KismetSystemLibrary.PrintString` "Match found!" true true (struct :`R` 1.0 :`G` 0.696735 :`A` 1.0))
    (`self.GetMatch`)))

(event `GetMatch`
  (`PlayFabMultiplayerAPI.GetMatch` (make `MultiplayerGetMatchRequest` :`MatchId` (`self.MatchId`) :`QueueName` (`self.QueueName`)) (delegate `SuccessGetMatch`) (`|CreateDelegate` :!event `OnFailure`)))

(event `SuccessGetMatch`
  (params (result :type "MultiplayerGetMatchResult Structure") (customData :type "Object Object Reference"))
  (bind (_matchid _members _regionpreferences _serverdetails) (break `MultiplayerGetMatchResult` result))
  (for _array_element _members
    (if (`KismetStringLibrary.EqualEqual_StrStr` (`PlayFabJsonObject.GetStringField` (`PlayFabJsonObject.GetObjectField` _array_element "Entity") "Id") (`.TitlePlayerAccountId_15_8D16608C408A11DCCB376A8CD5D80432` (break `/Game/BattleDronesMultiplayer/Blueprints/GameSettings/Utilities/S_UserAccount` (`self.UserAccount`))))
      (bind _returnvalue (`PlayFabJsonObject.GetStringField` _array_element "TeamId"))
      (switch `string` _returnvalue
        (:`team1`
          _)
        (:`team2`
          _))
      (bind _returnvalue_2 (`PlayFabJsonObject.GetObjectArrayField` _serverdetails "Ports"))
      (bind _returnvalue_3 (`KismetStringLibrary.Concat_StrStr` "Open " (`PlayFabJsonObject.GetStringField` _serverdetails "IPV4Address") ":" (`KismetStringLibrary.Conv_DoubleToString` (`PlayFabJsonObject.GetNumberField` (`|GetArrayItem` _returnvalue_2) "Num")) (`KismetStringLibrary.Concat_StrStr` "?Name=" (`.Username_5_2983CA96413BB83526A99099AE2D254F` (break `/Game/BattleDronesMultiplayer/Blueprints/GameSettings/Utilities/S_UserAccount` (`self.UserAccount`)))) (`KismetStringLibrary.Concat_StrStr` "?Team=" _returnvalue)))
      (`KismetSystemLibrary.PrintString` _returnvalue_3 true true (struct :`R` 0.766684 :`B` 1.0 :`A` 1.0) 5.0)
      (`KismetSystemLibrary.ExecuteConsoleCommand` _returnvalue_3 (`GameplayStatics.GetPlayerController` 0)))))

(event `CreateMatchmakingTicket`
  (`PlayFabMultiplayerAPI.CreateMatchmakingTicket` (make `MultiplayerCreateMatchmakingTicketRequest` :`Creator` (`self.CreatorSettings`) :`GiveUpAfterSeconds` 120 :`QueueName` (`self.QueueName`)) (delegate `SuccessCreateMatchmakingTicket`) (`|CreateDelegate` :!event `OnFailure`)))

(event `SuccessCancelAllMatchmakingTicketsForPlayer`
  (params (result :type "MultiplayerCancelAllMatchmakingTicketsForPlayerResult Structure") (customData :type "Object Object Reference"))
  (`self.CreateMatchmakingTicket`))

(event `AddCurrency`
  (`PlayFabClientAPI.ExecuteCloudScript` (make `ClientExecuteCloudScriptRequest` :`FunctionName` "addPlayerAD10") (delegate `SuccessAddCurrency`) (`|CreateDelegate` :!event `OnFailure`)))

(event `SuccessAddCurrency`
  (params (result :type "ClientExecuteCloudScriptResult Structure") (customData :type "Object Object Reference"))
  (`KismetSystemLibrary.PrintString` "You received reward successfully." true true (struct :`R` 1.0 :`G` 0.5 :`A` 1.0)))

(fn `CheckIfMatchFound`
  (`KismetSystemLibrary.PrintString` "Searching..." true true (struct :`G` 1.0 :`B` 0.5 :`A` 1.0) 4.5)
  (`self.GetMatchmakingTicket`))