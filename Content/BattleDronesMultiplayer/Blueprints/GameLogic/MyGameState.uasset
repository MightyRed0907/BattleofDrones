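; Game state for the BattleDrones multiplayer game, holding match status, selection and game timers, team scores and the result.
; It exposes plain getters and setters, with no match logic of its own.
; Points are read and incremented per team for teams A and B, and the result pairs a winning team with a draw flag.
; The game timer getter returns the remaining seconds formatted as minutes and seconds, or "0:00" once expired.
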(fn `Add Points`
  (params (Team :type "/Game/BattleDronesMultiplayer/Blueprints/GameLogic/Utilities/Teams Enum" :default "NewEnumerator0"))
  (switch `/Game/BattleDronesMultiplayer/Blueprints/GameLogic/Utilities/Teams` Team
    (:`NewEnumerator0`
      (`/Engine/EditorBlueprintResources/StandardMacros.IncrementInt` (`self.Team A Points`)))
    (:`NewEnumerator1`
      (`/Engine/EditorBlueprintResources/StandardMacros.IncrementInt` (`self.Team B Points`)))))

(fn `Get Game Status`
  (returns (`Return Value` :type "/Game/BattleDronesMultiplayer/Blueprints/GameLogic/Utilities/GameStatus Enum"))
  (return (`self.Game Status`)))

(fn `Get Game Timer`
  (returns (`Game Timer` :type Text))
  (bind _game_timer (`self.Game Timer`))
  (if (> _game_timer 0.0)
    (return (`KismetTextLibrary.AsTimespan_Timespan` (`KismetMathLibrary.MakeTimespan` 0 0 (`KismetMathLibrary.FFloor` (/ _game_timer 60.0)) (`KismetMathLibrary.FFloor` (mod _game_timer 60.0)))))
    (else
      (return "0:00"))))

(fn `Get Points`
  (params (Team :type "/Game/BattleDronesMultiplayer/Blueprints/GameLogic/Utilities/Teams Enum" :default "NewEnumerator0"))
  (returns (Points :type Integer))
  (switch `/Game/BattleDronesMultiplayer/Blueprints/GameLogic/Utilities/Teams` Team
    (:`NewEnumerator0`
      (return (`self.Team A Points`)))
    (:`NewEnumerator1`
      (return (`self.Team B Points`)))))

(fn `Get Selection TImer`
  (returns (`Selection Timer` :type "Float (double-precision)"))
  (return (`self.Selection Timer`)))

(fn `Get Winning Team`
  (returns (`Winning team` :type "/Game/BattleDronesMultiplayer/Blueprints/GameLogic/Utilities/Teams Enum") (Draw :type Boolean))
  (return (`self.Winning team`) (`self.Draw`)))

(fn `Set Game Status`
  (params (`New Game Status` :type "/Game/BattleDronesMultiplayer/Blueprints/GameLogic/Utilities/GameStatus Enum" :default "NewEnumerator0"))
  (set `self.Game Status` `New Game Status`))

(fn `Set Game Timer`
  (params (`Game Timer` :type "Float (double-precision)"))
  (set `self.Game Timer` `Game Timer`))

(fn `Set Selection Timer`
  (params (`Selection Timer` :type "Float (double-precision)"))
  (set `self.Selection Timer` `Selection Timer`))

(fn `Set Winning Team`
  (params (`Winning Team` :type "/Game/BattleDronesMultiplayer/Blueprints/GameLogic/Utilities/Teams Enum" :default "NewEnumerator0") (Draw :type Boolean))
  (set `self.Winning team` `Winning Team`)
  (set `self.Draw` Draw))

(fn `UserConstructionScript`)