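; Game mode for a two-team multiplayer drone battle, running matches from lobby through drone selection, play and end.
; Logins are balanced across teams; once enough players join, chained timers drive selection, spawning at random team starts and match duration.
; Tick copies remaining times to MyGameState and checks score limit or team dropout, while timeout compares points for winner or draw.
; An empty dedicated server quits after a short delay.
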(fn `Check Team Dropout`
  (bind _return_value (`self.Get My Game State`))
  (`|ExecutionSequence`
    (:`then_0`
      (if (<= (`self.Team A amount`) 0)
        (`/Game/BattleDronesMultiplayer/Blueprints/GameLogic/MyGameState.Set Winning Team` _return_value "NewEnumerator1" false)
        (`/Game/BattleDronesMultiplayer/Blueprints/GameLogic/MyGameState.Set Game Status` (`self.Get My Game State`) "NewEnumerator3" :!label _label)
        (`self.EndMatch`)))
    (:`then_1`
      (if (<= (`self.Team B amount`) 0)
        (`/Game/BattleDronesMultiplayer/Blueprints/GameLogic/MyGameState.Set Winning Team` _return_value "NewEnumerator0" false)
        (goto _label)))))

(fn `Check Win`
  (returns (ReturnValue :type Boolean))
  (bind _return_value (`self.Get My Game State`))
  (bind ((`PointsneededtoWin_9_B4163FDB41656377A65A6C92AC402517` _pointsneededtowin)) (break `/Game/BattleDronesMultiplayer/Blueprints/GameSettings/Utilities/GameSettings` (`/Game/BattleDronesMultiplayer/Blueprints/GameSettings/Utilities/GetGameSettings.Get Game Settings`)))
  (return (or (>= (`/Game/BattleDronesMultiplayer/Blueprints/GameLogic/MyGameState.Get Points` _return_value "NewEnumerator0") _pointsneededtowin) (>= (`/Game/BattleDronesMultiplayer/Blueprints/GameLogic/MyGameState.Get Points` _return_value "NewEnumerator1") _pointsneededtowin))))

(fn `Check Winning Team`
  (bind _return_value (`self.Get My Game State`))
  (bind _return_value_2 (`self.Get My Game State`))
  (bind _points (`/Game/BattleDronesMultiplayer/Blueprints/GameLogic/MyGameState.Get Points` _return_value_2 "NewEnumerator0"))
  (bind _points_2 (`/Game/BattleDronesMultiplayer/Blueprints/GameLogic/MyGameState.Get Points` _return_value_2 "NewEnumerator1"))
  (`/Game/BattleDronesMultiplayer/Blueprints/GameLogic/MyGameState.Set Game Status` (`self.Get My Game State`) "NewEnumerator3")
  (`self.EndMatch`)
  (if (== _points _points_2)
    (`/Game/BattleDronesMultiplayer/Blueprints/GameLogic/MyGameState.Set Winning Team` (`self.Get My Game State`) "NewEnumerator0" true)
    (elif (> _points _points_2)
      (`/Game/BattleDronesMultiplayer/Blueprints/GameLogic/MyGameState.Set Winning Team` _return_value "NewEnumerator0" false)
      (else
        (`/Game/BattleDronesMultiplayer/Blueprints/GameLogic/MyGameState.Set Winning Team` _return_value "NewEnumerator1" false)))))

(fn `Get My Game State`
  (returns (`Return Value` :type "/Game/BattleDronesMultiplayer/Blueprints/GameLogic/MyGameState Object Reference"))
  (bind _asmy_game_state (cast `/Game/BattleDronesMultiplayer/Blueprints/GameLogic/MyGameState` (`GameplayStatics.GetGameState`)))
  (return _asmy_game_state))

(fn `PrepareToStart`
  (`/Game/BattleDronesMultiplayer/Blueprints/GameLogic/MyGameState.Set Game Status` (`self.Get My Game State`) "NewEnumerator5")
  (`KismetSystemLibrary.K2_SetTimer` null "SpawningDrones" 3.0))

(fn `Spawn Drones`
  (params (`New Player Controller` :type "/Game/BattleDronesMultiplayer/Blueprints/Drones/DroneBase/MyPlayerController Object Reference") (`New Team` :type "/Game/BattleDronesMultiplayer/Blueprints/GameLogic/Utilities/Teams Enum" :default "NewEnumerator0") (`New Drone Class` :type "/Game/BattleDronesMultiplayer/Blueprints/Drones/DroneBase/DroneBase Class Reference") (`New Name` :type Text))
  (locals (`Local Player Controller` :type "/Game/BattleDronesMultiplayer/Blueprints/Drones/DroneBase/MyPlayerController Object Reference") (`Local Team` :type "/Game/BattleDronesMultiplayer/Blueprints/GameLogic/Utilities/Teams Enum" :default "NewEnumerator0") (`Local Drone Selected` :type "/Game/BattleDronesMultiplayer/Blueprints/Drones/DroneBase/DroneBase Class Reference") (`Local Player Name` :type Text))
  (set `local.Local Player Controller` `New Player Controller`)
  (set `local.Local Team` `New Team`)
  (set `local.Local Drone Selected` `New Drone Class`)
  (set `local.Local Player Name` `New Name`)
  (bind _outactors (`GameplayStatics.GetAllActorsOfClass` (`|GetArrayItem` (`self.PlayerStarts`) (`KismetMathLibrary.Conv_ByteToInt` (`local.Local Team`)))))
  (bind _returnvalue (`|SpawnActorFromClass` (`local.Local Drone Selected`) (`KismetMathLibrary.Conv_VectorToTransform` (`self.K2_GetActorLocation` (`|GetArrayItem` _outactors (`KismetMathLibrary.RandomIntegerInRange` 0 (- (`KismetArrayLibrary.Array_Length` _outactors) 1))))) "AdjustIfPossibleButAlwaysSpawn" "OverrideRootScale" null (`local.Local Player Name`) (`local.Local Team`) null))
  (`Controller.Possess` (`local.Local Player Controller`) _returnvalue))

(fn `SpawningDrones`
  (for _array_element (`self.All Player Connected`)
    (bind _asmy_player_state (cast `/Game/BattleDronesMultiplayer/Blueprints/Drones/DroneBase/MyPlayerState` (`Controller.PlayerState` _array_element)))
    (`self.Spawn Drones` _array_element (`/Game/BattleDronesMultiplayer/Blueprints/Drones/DroneBase/MyPlayerController.Get Team` _array_element) (`/Game/BattleDronesMultiplayer/Blueprints/Drones/DroneBase/MyPlayerController.Get Selected Drone` _array_element) (`/Game/BattleDronesMultiplayer/Blueprints/GameSettings/Utilities/GetGameSettings.Get Player Name` _asmy_player_state)))
  (`/Game/BattleDronesMultiplayer/Blueprints/GameLogic/MyGameState.Set Game Status` (`self.Get My Game State`) "NewEnumerator2")
  (bind _returnvalue (`KismetSystemLibrary.K2_SetTimer` null "StartGame" (`.GameDuration_7_7114F1E24999D8EA780C88A6036800C0` (break `/Game/BattleDronesMultiplayer/Blueprints/GameSettings/Utilities/GameSettings` (`/Game/BattleDronesMultiplayer/Blueprints/GameSettings/Utilities/GetGameSettings.Get Game Settings`)))))
  (set `self.Game Timer` _returnvalue))

(fn `StartGame`
  (`self.Check Winning Team`)
  (`self.StartMatch`))

(fn `UserConstructionScript`)