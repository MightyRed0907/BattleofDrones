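; Base pickup actor for multiplayer drones, with a rotating mesh and an overlap sphere that calls an empty ApplyEffect hook on the server.
; StartPickupRespawn hides the mesh, disables collision, enables tick and starts a timer that calls Respawn to reverse those changes.
; While the timer runs, the server's tick sets TimerValue to the elapsed fraction, and its RepNotify feeds a Percent material parameter on the base mesh to show respawn progress.
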(fn `Apply Effect`
  (params (`New Drone` :type "/Game/BattleDronesMultiplayer/Blueprints/Drones/DroneBase/DroneBase Object Reference")))

(fn `OnRep_Timer Value`
  (bind _pickup_base (`self.Pickup Base`))
  (bind _returnvalue (`PrimitiveComponent.CreateDynamicMaterialInstance` _pickup_base 1 (`PrimitiveComponent.GetMaterial` _pickup_base 1) "None"))
  (`MaterialInstanceDynamic.SetScalarParameterValue` _returnvalue "Percent" (`self.Timer Value`)))

(fn `Respawn`
  (`SceneComponent.SetVisibility` (`self.Pickup Mesh`) true false)
  (`PrimitiveComponent.SetCollisionEnabled` (`self.Sphere`) "QueryOnly")
  (`self.SetActorTickEnabled` false))

(fn `Start Pickup Respawn`
  (`self.SetActorTickEnabled` true)
  (`SceneComponent.SetVisibility` (`self.Pickup Mesh`) false false)
  (`PrimitiveComponent.SetCollisionEnabled` (`self.Sphere`) "NoCollision")
  (bind _returnvalue (`KismetSystemLibrary.K2_SetTimer` null "Respawn" (`self.Timer to Respawn`)))
  (set `self.Pickup Handle` _returnvalue))

(fn `UserConstructionScript`)