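; PickupReload is a pickup that grants a drone a temporary reload reduction.
; On ApplyEffect it asks the drone whether it can take the boost, then starts the reduction for ReloadDuration and begins the pickup's respawn.
; If the drone cannot take it, nothing happens and no respawn starts.
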(event `self.Apply Effect`
  (params (`New Drone` :type "/Game/BattleDronesMultiplayer/Blueprints/Drones/DroneBase/DroneBase Object Reference"))
  (if (`/Game/BattleDronesMultiplayer/Blueprints/Drones/DroneBase/DroneBase.Can Pickup Reload Reduction` `New Drone`)
    (`/Game/BattleDronesMultiplayer/Blueprints/Drones/DroneBase/DroneBase.Start Reload Reduction` `New Drone` (`self.Reload Duration`))
    (`self.Start Pickup Respawn`)))

(fn `UserConstructionScript`
  (`parent.UserConstructionScript`))